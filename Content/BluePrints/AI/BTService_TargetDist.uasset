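; Behavior Tree service that keeps the AI's distance to its target up to date in the Blackboard.
; On each AI tick it reads SelfActor and TargetActor from the Blackboard, casts both to Character, and writes the distance between their locations to TargetDist.
; If either cast fails, the tick stops without updating the value.
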(event `self.ReceiveTickAI`
  (params (OwnerController :type "AIController Object Reference") (ControlledPawn :type "Pawn Object Reference") (DeltaSeconds :type "Float (single-precision)"))
  (bind _returnvalue (`AIBlueprintHelperLibrary.GetBlackboard` OwnerController))
  (bind _ascharacter (cast `Character` (`BlackboardComponent.GetValueAsObject` (`AIBlueprintHelperLibrary.GetBlackboard` OwnerController) (`self.SelfActor`))))
  (bind _ascharacter_2 (cast `Character` (`BlackboardComponent.GetValueAsObject` _returnvalue (`self.TargetActor`))))
  (`BlackboardComponent.SetValueAsFloat` _returnvalue (`self.TargetDist`) (`KismetMathLibrary.Vector_Distance` (`Actor.K2_GetActorLocation` _ascharacter) (`Actor.K2_GetActorLocation` _ascharacter_2))))