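; AI controller for enemies that runs the BT_Enemy behavior tree on possession and tracks the player through AI perception.
; Sensing an actor tagged Player cancels the pending forget timer and writes that actor to the TargetActor blackboard key.
; Any other perception update starts a timer of LineOfSightTimer length, which empties TargetActor when it expires, giving a grace period after losing sight.
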(event `self.ReceivePossess`
  (params (PossessedPawn :type "Pawn Object Reference"))
  (`self.RunBehaviorTree` "/Game/BluePrints/AI/BT_Enemy.BT_Enemy")
  (`KismetSystemLibrary.K2_ClearAndInvalidateTimerHandle` (`self.EnemyTimer`) :!label _label)
  (`BlackboardComponent.SetValueAsObject` (`self.Blackboard`) (`self.TargetActor`) (stale `self.AIPerception.OnTargetPerceptionUpdated` Actor)))

(event `self.AIPerception.OnTargetPerceptionUpdated`
  (params (Actor :type "Actor Object Reference") (Stimulus :type "AIStimulus Structure"))
  (if (and (`self.ActorHasTag` Actor "Player") (`.bSuccessfullySensed` (break `AIStimulus` Stimulus)))
    (goto _label)
    (else
      (bind _returnvalue (`KismetSystemLibrary.K2_SetTimerDelegate` (delegate `StartEnemyTimer`) (`self.LineOfSightTimer`)))
      (set `self.EnemyTimer` _returnvalue))))

(event `StartEnemyTimer`
  (`BlackboardComponent.SetValueAsObject` (`self.Blackboard`) (`self.TargetActor`) null))

(fn `UserConstructionScript`)