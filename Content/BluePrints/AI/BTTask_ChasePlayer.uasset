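; Behavior tree task that makes an Enemy chase the character stored as the blackboard's target.
; Each AI tick it casts SelfActor to Enemy and TargetActor to Character, stopping if either cast fails.
; It then feeds the straight-line offset between them into AddMovementInput, with no pathfinding.
; The task never calls Finish Execute, so it does not end on its own.
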(event `self.ReceiveTickAI`
  (params (OwnerController :type "AIController Object Reference") (ControlledPawn :type "Pawn Object Reference") (DeltaSeconds :type "Float (single-precision)"))
  (bind _returnvalue (`AIBlueprintHelperLibrary.GetBlackboard` OwnerController))
  (bind _asenemy (cast `Enemy` (`BlackboardComponent.GetValueAsObject` _returnvalue (`self.SelfActor`))))
  (bind _ascharacter (cast `Character` (`BlackboardComponent.GetValueAsObject` _returnvalue (`self.TargetActor`))))
  (`Pawn.AddMovementInput` _asenemy (- (`Actor.K2_GetActorLocation` _ascharacter) (`Actor.K2_GetActorLocation` _asenemy)) 1.0 false))